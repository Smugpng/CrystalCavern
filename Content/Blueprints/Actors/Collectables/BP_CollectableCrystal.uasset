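; Collectable crystal actor that flies into the player pawn and vanishes when the player overlaps it.
; On overlap it caches its location, scale and point light intensity, then plays a timeline.
; Separate timeline tracks drive lerps that pull it toward the pawn's live location, shrink it to zero and fade the light out.
; The actor destroys itself when the timeline finishes; no score or inventory update happens here.
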(event `self.ReceiveActorBeginOverlap`
  (params (OtherActor :type "Actor Object Reference"))
  (if (== OtherActor (`GameplayStatics.GetPlayerPawn` 0))
    (`self.Store Starting Values`)
    (bind (_direction _collection_progress _scale_progress _light_intesnsity) (`Timeline|Collection timeline`)
      (:`Update`
        (`self.MoveTowardsPlayer` _collection_progress)
        (`self.NewFunction` _scale_progress)
        (`self.NewFunction_0` _light_intesnsity))
      (:`Finished`
        (`self.K2_DestroyActor`)))))

(fn `MoveTowardsPlayer`
  (params (Alpha :type "Float (single-precision)"))
  (`self.K2_SetActorLocation` (`KismetMathLibrary.VLerp` (`self.Start Location`) (`self.K2_GetActorLocation` (`GameplayStatics.GetPlayerPawn` 0)) Alpha)))

(fn `NewFunction`
  (params (Alpha :type "Float (single-precision)"))
  (`self.SetActorScale3D` (`KismetMathLibrary.VLerp` (`self.StartScale`) (0.0 0.0 0.0) Alpha)))

(fn `NewFunction_0`
  (params (Alpha :type "Float (double-precision)"))
  (`LightComponent.SetIntensity` (`self.PointLight`) (`KismetMathLibrary.Lerp` (`self.Start Light Intensity`) 0.0 Alpha)))

(fn `Store Starting Values`
  (set `self.Start Location` (`self.K2_GetActorLocation`))
  (set `self.StartScale` (`self.GetActorScale3D`))
  (set `self.Start Light Intensity` (`LightComponentBase.Intensity` (`self.PointLight`))))

(fn `UserConstructionScript`)